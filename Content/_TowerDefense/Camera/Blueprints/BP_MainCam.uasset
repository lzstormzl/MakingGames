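; BP_MainCam is the tower defense main camera, carrying map fog-of-war hooks on BeginPlay and Tick that currently do nothing.
; Both fog events are empty, and the logic meant for them sits disconnected.
; That unwired logic clears two render targets and creates fog and reveal dynamic materials with a reveal radius.
; It also traces vertically through the actor, converts the hit to UVs, and draws both materials into the targets there.
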(event Custom|Fog_Tick)

(event Custom|Fog_Begin)

(event EventBeginPlay
  (Utilities|FlowControl|Sequence
    (:then_0
      (CallFunction|FogBegin))))

(event EventTick
  (params (DeltaSeconds :type Float%20%28single-precision%29))
  (CallFunction|FogTick))

(fn ConstructionScript)