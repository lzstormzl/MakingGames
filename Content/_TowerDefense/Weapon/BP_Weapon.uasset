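; BP_Weapon is a projectile actor that homes in on a given enemy and deals physical damage.
; On BeginPlay it attaches the NS_Projectile Niagara effect to its Projectile component.
; FCastProjectile, called from the character, stores the target and runs the FlyToEnemy timeline, lerping from current location toward the enemy's live position.
; Sphere overlap with that target sends damage combining player and projectile stats plus armor reduction, then destroys the actor and deactivates the effect.
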(event OnComponentBeginOverlap(Sphere)
  (params (OverlappedComponent :type Primitive%20Component%20Object%20Reference) (OtherActor :type Actor%20Object%20Reference) (OtherComp :type Primitive%20Component%20Object%20Reference) (OtherBodyIndex :type Integer) (bFromSweep :type Boolean) (SweepResult :type Hit%20Result%20Structure%20%28by%20ref%29))
  (if (== OtherActor (Variables|Default|GetDamaged_Enemy))
    (Class|BPIEnemy|ETakePhysDmg(Message) (Variables|Default|GetDamaged_Enemy) (CallFunction|FPlayerTotalPhysicDmg (Variables|Default|GetPlayer_Dmg (Variables|Default|GetBPC_PlayerStats)) (Variables|/Game/_TowerDefense/Weapon/BPC_Weapon.BPC_Weapon_C|GetDamage (Variables|Default|GetBPC_ProjectileStats))) (Variables|/Game/_TowerDefense/Weapon/BPC_Weapon.BPC_Weapon_C|GetReduce%20Armor (Variables|Default|GetBPC_ProjectileStats)) 0.0)
    (Actor|DestroyActor)
    (CallFunction|DeactiveNSCE)))

(event Custom|Deactive_NS_CE
  (Utilities|IsValid (stale EventBeginPlay _returnvalue)
    (:Is%20Valid
      (Components|Activation|Deactivate (stale EventBeginPlay _returnvalue)))))

(event EventBeginPlay
  (bind _projectile (Variables|Default|GetProjectile))
  (Utilities|FlowControl|Sequence
    (:then_1
      (bind _returnvalue (Niagara|SpawnSystemAttached "/Game/_TowerDefense/Weapon/Fx/NS_Projectile.NS_Projectile" _projectile "None" (Transformation|GetWorldLocation _projectile) "0, 0, 0" "KeepRelativeOffset" false)))))

(event Collision|EventActorBeginOverlap
  (params (OtherActor :type Actor%20Object%20Reference)))

(event EventTick
  (params (DeltaSeconds :type Float%20%28single-precision%29)))

(event EventFCastProjectile
  (params (EnemyActor :type Actor%20Object%20Reference))
  (Utilities|IsValid EnemyActor
    (:Is%20Valid
      (Variables|Default|SetDamaged_Enemy EnemyActor)
      (bind _alpha (Timeline|FlyToEnemy PlayFromStart)
        (:Update
          (Transformation|SetActorLocation (Math|Vector|Lerp(Vector) (Transformation|GetActorLocation) (Transformation|GetActorLocation (Variables|Default|GetDamaged_Enemy)) _alpha) false false))))))

(fn ConstructionScript)