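; BP_AllyBase is the base ally unit for the tower defense game, handling click selection and move orders.
; Clicking the unit toggles a FlipFlop that shows or hides its selection UI and notifies player controller 0 through interface messages that it was selected or deselected.
; An interface Goto event receives a destination and sends the unit there with AIMoveTo.
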(event EventBeginPlay)

(event Collision|EventActorBeginOverlap
  (params (OtherActor :type Actor%20Object%20Reference)))

(event EventTick
  (params (DeltaSeconds :type Float%20%28single-precision%29)))

(event MouseInput|EventActorOnClicked
  (params (ButtonPressed :type Key%20Structure :default "None"))
  (Utilities|FlowControl|FlipFlop
    (:A
      (Development|SetHiddeninGame (Variables|Default|GetSelectedActor_UI) false false)
      (Class|BPICamSelectAllyUnit|SelectedBPICamselectAllyUnit(Message) (Game|GetPlayerController 0) self))
    (:B
      (Development|SetHiddeninGame (Variables|Default|GetSelectedActor_UI) true false)
      (Class|BPICamSelectAllyUnit|DeSelectedBPICamselectAllyUnit(Message) (Game|GetPlayerController 0) self))))

(event EventGotoBPIAllyUnit
  (params (Destination :type Vector :default "0, 0, 0"))
  (AI|AIMoveTo self Destination 0 5.0 false))

(fn ConstructionScript)