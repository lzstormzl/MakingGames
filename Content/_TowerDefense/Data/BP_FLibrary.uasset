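; Blueprint function library of physical damage formulas for the tower defense game.
; Total damage is the sum of player and weapon damage.
; HP loss subtracts effective armor (enemy armor less armor reduction) scaled by a per-armor factor, with a floor of 1.
; A random roll varies configured damage downward only, by up to a given percentage.
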(fn FPlayerTotalPhysicDmg
  (params (Player_Dmg :type Float%20%28double-precision%29) (Weapon_Dmg :type Float%20%28double-precision%29))
  (return (+ Player_Dmg Weapon_Dmg)))

(fn FPhysicDmgHPLoss
  (params (Total%20PhysicDmg :type Float%20%28double-precision%29) (Enemy_Armor :type Float%20%28double-precision%29) (Reduce_Armor_Eff :type Float%20%28double-precision%29))
  (bind _returnvalue (- Enemy_Armor Reduce_Armor_Eff))
  (bind _dmg_reduce_perarmor (LocalVariables|GetDmg_Reduce_PerArmor))
  (bind _returnvalue_2 (* _returnvalue _dmg_reduce_perarmor))
  (bind _returnvalue_3 (- Total%20PhysicDmg _returnvalue_2))
  (if (> _returnvalue_3 1.0)
    (return _returnvalue_3)
    (else
      (return 1.0))))

(fn FRdmRangePhysicDmg
  (params (Dmg_Config :type Float%20%28double-precision%29) (Range_Rdm_Ratio :type Float%20%28double-precision%29))
  (return (Math|Random|RandomFloatinRange (* Dmg_Config (- 1.0 (/ Range_Rdm_Ratio 1e+02))) Dmg_Config)))