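; Enemy spawner actor for a tower defense game that spawns small and big enemies at random reachable navmesh points around itself.
; BeginPlay requests an initial small spawn and starts two looping timers, one per enemy type.
; The spawn events increment a counter for their type and clear the matching timer handle when that counter equals its maximum.
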(event Custom|SpawnSmall_Enemy
  (Game|SpawnActorfromClass "/Game/_TowerDefense/Evemy/BP_Enemy.BP_Enemy_C" (Math|Transform|MakeTransform (.RandomLocation (AI|Navigation|GetRandomReachablePointinRadius (Transformation|GetActorLocation) 1e+03 0 0)) "0, 0, 0" "1.000000,1.000000,1.000000") "Undefined" "MultiplyWithRoot" 0 0)
  (Math|Integer|IncrementInt (Variables|SmallE1|GetSmall_E_Number)
    (:%20%20
      (if (== (Variables|Small_E1|GetSmall_E_Max) (Variables|SmallE1|GetSmall_E_Number))
        (Utilities|Time|ClearandInvalidateTimerbyHandle (Variables|SmallE1|GetSpawn_E1_TimerHandle))))))

(event Custom|SpawnBig_Enemy
  (Game|SpawnActorfromClass "/Game/_TowerDefense/Evemy/BP_BigEnemy.BP_BigEnemy_C" (Math|Transform|MakeTransform (.RandomLocation (AI|Navigation|GetRandomReachablePointinRadius (Transformation|GetActorLocation) 1e+03 0 0)) "0, 0, 0" "1.000000,1.000000,1.000000") "Undefined" "MultiplyWithRoot" 0 0)
  (Math|Integer|IncrementInt (Variables|BigE1|GetSmall_Big_E_Number)
    (:%20%20
      (if (== (Variables|BigE1|GetSmall_BigE_Max) (Variables|BigE1|GetSmall_Big_E_Number))
        (Utilities|Time|ClearandInvalidateTimerbyHandle (Variables|Big_E1|GetSpawn_BigE1_TimerHandle))))))

(event EventBeginPlay
  (CallFunction|SpawnSmallEnemy)
  (bind _returnvalue (Utilities|Time|SetTimerbyEvent (EventDispatchers|CreateEvent :!event Custom|SpawnSmall_Enemy) 2.5 true))
  (Variables|SmallE1|SetSpawn_E1_TimerHandle _returnvalue)
  (bind _returnvalue_2 (Utilities|Time|SetTimerbyEvent (EventDispatchers|CreateEvent :!event Custom|SpawnBig_Enemy) 2.5 true))
  (Variables|Big_E1|SetSpawn_BigE1_TimerHandle _returnvalue_2))

(event Collision|EventActorBeginOverlap
  (params (OtherActor :type Actor%20Object%20Reference)))

(event EventTick
  (params (DeltaSeconds :type Float%20%28single-precision%29)))

(fn ConstructionScript)