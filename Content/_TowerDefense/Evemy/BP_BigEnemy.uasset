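; Big enemy for the tower defense game that chases the player character with AI MoveTo, stopping at a wide acceptance radius.
; BeginPlay starts the chase and a looping timer, then loads HP from the enemy stats component.
; An interface damage event applies armor-adjusted damage, either reducing HP or destroying the enemy and notifying the player of the death.
; The face-the-player rotation logic is disconnected and never runs.
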(event Custom|ChasePlayer
  (AI|AIMoveTo self "0, 0, 0" (Game|GetPlayerCharacter 0) 8e+02 false))

(event Custom|LockRotation)

(event EventBeginPlay
  (Utilities|FlowControl|Sequence
    (:then_0
      (CallFunction|ChasePlayer)
      (Utilities|Time|SetTimerbyEvent (EventDispatchers|CreateEvent :!event Custom|LockRotation) 0.1 true))
    (:then_1
      (|Stats))))

(event EventFETakeDmgBPIEnemy
  (params (Total_Dmg :type Float%20%28double-precision%29) (Reduce_Armor :type Float%20%28double-precision%29) (Reduce_Magic_Resist :type Float%20%28double-precision%29))
  (bind _bc_enemystats_comp (Variables|Default|GetBC_EnemyStats_Comp))
  (bind _big_e1_armor (Variables|/Game/_TowerDefense/Evemy/Component/BC_EnemyStats_Comp.BC_EnemyStats_Comp_C|GetBig_E1_Armor _bc_enemystats_comp))
  (bind _hp_loss (CallFunction|FPhysicDmgHPLoss Total_Dmg _big_e1_armor Reduce_Armor))
  (if (>= _hp_loss (Variables|Default|GetEnemyHP))
    (Actor|DestroyActor)
    (Class|BPIPlayer|FEnemyDie?BPIPlayer(Message) (Game|GetPlayerCharacter 0))
    (else
      (Variables|Default|SetEnemyHP (- (Variables|Default|GetEnemyHP) _hp_loss))
      (Development|PrintString (Utilities|String|ToString(Float) _hp_loss) true true "(R=0.068439,G=0.000000,B=1.000000,A=1.000000)" 2.0 "1"))))

(event EventTick
  (params (DeltaSeconds :type Float%20%28single-precision%29)))

(fn ConstructionScript)