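; Tower defense base character that automatically attacks enemies entering its range.
; RangeAtk overlap queues tagged enemies, and a looping timer drives the attack, turning the mesh toward the first one and playing a DoOnce-gated montage.
; An attack animation interface callback spawns a BP_Projectile, passes it that target, then re-arms the montage after an AtkSpeed delay.
; An enemy-death interface event drops the first queue entry; nothing removes enemies leaving range.
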(event OnComponentBeginOverlap(RangeAtk)
  (params (OverlappedComponent :type Primitive%20Component%20Object%20Reference) (OtherActor :type Actor%20Object%20Reference) (OtherComp :type Primitive%20Component%20Object%20Reference) (OtherBodyIndex :type Integer) (bFromSweep :type Boolean) (SweepResult :type Hit%20Result%20Structure%20%28by%20ref%29))
  (if (Actor|ActorHasTag OtherActor "Enemy")
    (Utilities|Array|AddUnique (Variables|Default|GetEnemyOnRangeAtk) OtherActor)))

(event Custom|Attack%20Enemy_CE
  (if (> (Utilities|Array|Length (Variables|Default|GetEnemyOnRangeAtk)) 0)
    (Utilities|FlowControl|Sequence
      (:then_0
        (CallFunction|AnimAtkCE))
      (:then_1
        (CallFunction|RotatetoEnemyCE)))))

(event Custom|Rotate_ToEnemy_CE
  (bind _self self)
  (bind _enemyonrangeatk (Variables|Default|GetEnemyOnRangeAtk))
  (bind _returnvalue (Transformation|GetActorLocation _self))
  (bind _output (Utilities|Array|Get(acopy) _enemyonrangeatk))
  (bind _returnvalue_2 (Transformation|GetActorLocation _output))
  (bind _returnvalue_3 (Math|Rotator|FindLookatRotation _returnvalue _returnvalue_2))
  (Transformation|SetRelativeRotation (Variables|Character|GetMesh) (Math|Rotator|MakeRotator (.roll _returnvalue_3) 0.0 (+ (.yaw _returnvalue_3) 9e+01)) false false))

(event Custom|Anim_Atk_CE
  (Utilities|FlowControl|DoOnce false
    (:Completed
      (Animation|Montage|PlayMontage (Variables|Character|GetMesh) "/Game/_TowerDefense/Player/Base/Anim/ChrBase_Atk_Montage.ChrBase_Atk_Montage"))))

(event Custom|Reset_Atk_Anim_CE
  (Utilities|FlowControl|DoOnce false) ; enters at Reset
)

(event EventBeginPlay
  (Utilities|Time|SetTimerbyEvent (EventDispatchers|CreateEvent :!event Custom|Attack%20Enemy_CE) 0.1 true) ; Chạy Cus Event tấn công, bao gồm nhìn Enemy và Anim tấn công
)

(event Collision|EventActorBeginOverlap
  (params (OtherActor :type Actor%20Object%20Reference)))

(event EventTick
  (params (DeltaSeconds :type Float%20%28single-precision%29)))

(event EventFAtkEBPIPlayer
  (bind _returnvalue (Game|SpawnActorfromClass "/Game/_TowerDefense/Projectile/BP_Projectile.BP_Projectile_C" (Math|Transform|MakeTransform (Transformation|GetWorldLocation (Variables|Character|GetMesh)) "0, 0, 0" "1.000000,1.000000,1.000000") "Undefined" "MultiplyWithRoot" 0 0))
  (Class|BPIPlayerProjectile|FCastProjectileBPIProjectile(Message) _returnvalue (Utilities|Array|Get(acopy) (Variables|Default|GetEnemyOnRangeAtk))) ; Cast đến BP Projectile để Active
  (Utilities|FlowControl|Delay (Variables|Default|GetAtkSpeed))
  (CallFunction|ResetAtkAnimCE) ; Reset Anim tấn công
)

(event EventFEnemyDie?BPIPlayer
  (Utilities|Array|RemoveItem (Variables|Default|GetEnemyOnRangeAtk) (Utilities|Array|Get(acopy) (Variables|Default|GetEnemyOnRangeAtk))))

(fn ConstructionScript)